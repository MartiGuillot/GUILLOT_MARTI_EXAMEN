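; Door actor that swings its mesh open or closed based on player proximity and a coin requirement.
; FrameCollision overlaps toggle IsNearDoor without filtering the overlapping actor, while HasEnoughCoins is only read here, not set.
; Tick restarts DoorOpenerTimeline every frame, reversing from the end when both flags are true and playing from the start otherwise, with its track driving the mesh's relative yaw.
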(event OnComponentBeginOverlap(FrameCollision)
  (params (OverlappedComponent :type Primitive%20Component%20Object%20Reference) (OtherActor :type Actor%20Object%20Reference) (OtherComp :type Primitive%20Component%20Object%20Reference) (OtherBodyIndex :type Integer) (bFromSweep :type Boolean) (SweepResult :type Hit%20Result%20Structure%20%28by%20ref%29))
  ;[1 1 1] Near Door Detection
  (Variables|Default|SetisNearDoor true))

(event OnComponentEndOverlap(FrameCollision)
  (params (OverlappedComponent :type Primitive%20Component%20Object%20Reference) (OtherActor :type Actor%20Object%20Reference) (OtherComp :type Primitive%20Component%20Object%20Reference) (OtherBodyIndex :type Integer))
  ;[1 1 1] Near Door Detection
  (Variables|Default|SetisNearDoor false))

(event EventBeginPlay)

(event Collision|EventActorBeginOverlap
  (params (OtherActor :type Actor%20Object%20Reference)))

(event EventTick
  (params (DeltaSeconds :type Float%20%28single-precision%29))
  ;[1 1 1] Update (Door Opener)
  (if (and (Variables|Default|GetisNearDoor) (Variables|Default|GethasEnoughCoins))
    (bind _doortobeopenedamountrotate (Timeline|DoorOpenerTimeline ReverseFromEnd)
      (:Update
        (Transformation|SetRelativeRotation (Variables|Default|GetDoorMesh) (Math|Rotator|MakeRotator 0.0 0.0 _doortobeopenedamountrotate) false false)))
    (else
      (Timeline|DoorOpenerTimeline PlayFromStart))))

(fn ConstructionScript)